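; Pear tree crop that visually grows in two stages as crop growth progresses.
; The construction script collects static mesh components with "pear" in their names into FruitMeshes, so fruit is found by naming convention.
; SetPlantScaleBasedonGrowth maps the first half of growth progress to the tree's world scale and the second half to the fruit's, so pears swell once the tree reaches full size.
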(event `self.SetPlantScaleBasedOnGrowth`
  (bind _returnvalue (`self.GetCropGrowthProgress`))
  (bind _fruitscale (`self.FruitScale`))
  (bind _treescale (`self.TreeScale`))
  (set `self.TreeScale` (`KismetMathLibrary.Lerp` 0.0 0.3 (`KismetMathLibrary.FClamp` (* _returnvalue 2.0))))
  (set `self.FruitScale` (`KismetMathLibrary.Lerp` 0.0 1.0 (`KismetMathLibrary.FClamp` (* (- _returnvalue 0.5) 2.0))))
  (`SceneComponent.SetWorldScale3D` (`self.Tree`) (`KismetMathLibrary.MakeVector` _treescale _treescale _treescale))
  (for _array_element (`self.FruitMeshes`)
    (`SceneComponent.SetWorldScale3D` _array_element (`KismetMathLibrary.MakeVector` _fruitscale _fruitscale _fruitscale))))

(fn `UserConstructionScript`
  (for _array_element (`self.K2_GetComponentsByClass` "/Script/Engine.StaticMeshComponent")
    (if (`KismetStringLibrary.Contains` (`KismetSystemLibrary.GetObjectName` _array_element) "pear")
      (`KismetArrayLibrary.Array_Add` (`self.FruitMeshes`) _array_element))))