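; Tomato crop Blueprint that visually grows its vine and fruit meshes from the crop's growth progress.
; The construction script sorts static mesh components into sapling and tomato arrays by case-sensitive name substring.
; SetPlantScaleBasedonGrowth scales saplings to full size over the first half of growth, then grows tomatoes from zero to their smaller final scale over the second half.
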(event `self.SetPlantScaleBasedOnGrowth`
  (bind _returnvalue (`self.GetCropGrowthProgress`))
  (bind _tomatoscale (`self.TomatoScale`))
  (bind _vinescale (`self.VineScale`))
  (set `self.VineScale` (`KismetMathLibrary.FClamp` (* _returnvalue 2.0)))
  (set `self.TomatoScale` (`KismetMathLibrary.Lerp` 0.0 0.75 (`KismetMathLibrary.FClamp` (* (- _returnvalue 0.5) 2.0))))
  (for _array_element (`self.SaplingMeshes`)
    (`SceneComponent.SetWorldScale3D` _array_element (`KismetMathLibrary.MakeVector` _vinescale _vinescale _vinescale)))
  (for _array_element_2 (`self.TomatoMeshes`)
    (`SceneComponent.SetWorldScale3D` _array_element_2 (`KismetMathLibrary.MakeVector` _tomatoscale _tomatoscale _tomatoscale))))

(fn `UserConstructionScript`
  (for _array_element (`self.K2_GetComponentsByClass` "/Script/Engine.StaticMeshComponent")
    (bind _returnvalue (`KismetSystemLibrary.GetObjectName` _array_element))
    (if (`KismetStringLibrary.Contains` _returnvalue "Tomato" true)
      (`KismetArrayLibrary.Array_Add` (`self.TomatoMeshes`) _array_element)
      (elif (`KismetStringLibrary.Contains` _returnvalue "Sapling" true)
        (`KismetArrayLibrary.Array_Add` (`self.SaplingMeshes`) _array_element)))))